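; Mob spawner that runs round-based zombie waves, alternating timed rounds with short breaks and publishing round, timer and quota to GI_GI.
; Tick drives the timer and ZomSpawner, which spawns zombies at random nearby navmesh points until a round-scaled quota is passed.
; Fast and hard zombies join in later rounds, paced by modulo on a per-tick counter rather than seconds.
; Round end calls MobKiller to destroy zombies and flying enemies.
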(event Custom|MobSpawn
  (bind _lshspawnzomcounter (Variables|Default|GetLSHspawnZomCounter))
  ;[1 1 1] 라운드 참이고 라운드좀비총수 >= 스폰좀비수면 좀비 10 소환
  (if (Variables|Default|GetLSHIsRound)
    (if (>= (Variables|Default|GetLSHRoundZomNum) (Variables|Default|GetLSHspawnZomCounter))
      (CallFunction|MobMaker "/Game/SH_AI/NavigationSystem/BP_Zom.BP_Zom_C")
      (Math|Integer|IncrementInt _lshspawnzomcounter
        (:%20%20
          (Development|PrintString (Utilities|String|ToString(Integer) _lshspawnzomcounter)))))))

(event EventBeginPlay)

(event Collision|EventActorBeginOverlap
  (params (OtherActor :type Actor%20Object%20Reference)))

(event EventTick
  (params (DeltaSeconds :type Float%20%28single-precision%29))
  (bind _asgi_gi (Utilities|Casting|CastToGI_GI (Game|GetGameInstance)))
  (Variables|/Game/SH_AI/HUD/GI_GI.GI_GI_C|SetLSH_GI_RoundTime _asgi_gi (Math|Float|Truncate (Variables|Default|GetLSH_Timer)))
  (bind _result (Math|Integer|IncrementInt (Variables|Default|GetLSH_TimeCounter))
    (:%20%20
      (bind _asgi_gi_2 (Utilities|Casting|CastToGI_GI (Game|GetGameInstance)))
      (Variables|/Game/SH_AI/HUD/GI_GI.GI_GI_C|SetLSH_GI_Timer _asgi_gi_2 _result)
      (Variables|Default|SetLSH_currentTime (+ (Variables|Default|GetLSH_currentTime) DeltaSeconds))
      (CallFunction|ZomSpawner (Variables|Default|GetLSHround) (Variables|Default|GetLSHIsRound))
      (if (< (Variables|Default|GetLSH_Timer) (Variables|Default|GetLSH_currentTime))
        (if (Variables|Default|GetLSHIsRound)
          ;[1 1 1] 만약 라운드가 참이고 시간이 종료되었다면 라운드를 종료시키고 준비시간 20초 카운트
          (Variables|Default|SetLSH_currentTime 0.0)
          (Variables|Default|SetLSH_Timer 5.0)
          (Variables|Default|SetLSHIsRound false)
          (CallFunction|MobKiller)
          (Development|PrintString "라운드 종료")
          (Variables|Default|SetLSHspawnZomCounter 0)
          (Variables|Default|SetLSH_TimeCounter 0)
          (bind _asgi_gi_3 (Utilities|Casting|CastToGI_GI (Game|GetGameInstance)))
          (Variables|/Game/SH_AI/HUD/GI_GI.GI_GI_C|SetLSH_GI_RoundZomNum _asgi_gi_3 0)
          (else
            ;[1 1 1] 만약 라운드가 거짓이고 시간이 종료되었다면 라운드를 1증가시키고 시작시키고 라운드시간 180초 카운트
            (Variables|Default|SetLSH_currentTime 0.0)
            (Variables|Default|SetLSH_Timer 3e+01)
            (Variables|Default|SetLSHIsRound true)
            (Variables|Default|SetLSHRoundZomNum (+ (* (Variables|Default|GetLSHround) 12) (Variables|Default|GetLSHDefaultZomNum)))
            (bind _result_2 (Math|Integer|IncrementInt (Variables|Default|GetLSHround))
              (:%20%20
                (Development|PrintString (Utilities|String|Append (Utilities|String|ToString(Integer) _result_2) " 라운드 시작"))
                (Development|PrintString (Utilities|String|ToString(Integer) (Variables|Default|GetLSHRoundZomNum)))
                (Development|PrintString (Utilities|String|ToString(Integer) (Variables|Default|GetLSHspawnZomNum)))
                (Variables|Default|SetLSH_TimeCounter 0)
                (bind _asgi_gi_4 (Utilities|Casting|CastToGI_GI (Game|GetGameInstance)))
                (Variables|/Game/SH_AI/HUD/GI_GI.GI_GI_C|SetLSH_GI_RoundZomNum _asgi_gi_4 (Variables|Default|GetLSHRoundZomNum))
                (bind _asgi_gi_5 (Utilities|Casting|CastToGI_GI (Game|GetGameInstance)))
                (Variables|/Game/SH_AI/HUD/GI_GI.GI_GI_C|SetLSH_GI_Round _asgi_gi_5 (Variables|Default|GetLSHround))))))))))

(fn ConstructionScript)

(fn RoundStart
  (Variables|Default|SetLSHIsRound true)
  (CallFunction|MobSpawn))

(fn MobKiller
  (bind _outactors (Actor|GetAllActorsOfClass "/Game/SH_AI/NavigationSystem/BP_Zom.BP_Zom_C"))
  (Actor|DestroyActor _outactors)
  (bind _outactors_2 (Actor|GetAllActorsOfClass "/Game/SH_AI/NavigationSystem/BP_FastZom.BP_FastZom_C"))
  (Actor|DestroyActor _outactors_2)
  (bind _outactors_3 (Actor|GetAllActorsOfClass "/Game/SH_AI/NavigationSystem/BP_HardZom.BP_HardZom_C"))
  (Actor|DestroyActor _outactors_3)
  (bind _outactors_4 (Actor|GetAllActorsOfClass "/Game/JE_AI/BP_FlyingEnemyAI.BP_FlyingEnemyAI_C"))
  (Actor|DestroyActor _outactors_4)
  (bind _asgi_gi (Utilities|Casting|CastToGI_GI (Game|GetGameInstance)))
  (Variables|/Game/SH_AI/HUD/GI_GI.GI_GI_C|SetLSH_GI_RoundZomNum _asgi_gi 0))

(fn MobMaker
  (params (LSH_zomClass :type Actor%20Class%20Reference))
  (bind _returnvalue (Game|SpawnActorfromClass LSH_zomClass (Math|Conversions|ToTransform(Vector) (.RandomLocation (AI|Navigation|GetRandomReachablePointinRadius (Transformation|GetActorLocation) 5e+02 0 0))) "Undefined" "MultiplyWithRoot" 0 0))
  (Pawn|SpawnDefaultController (Variables|/Script/Engine.Actor|GetInstigator _returnvalue))
  (Math|Integer|IncrementInt (Variables|Default|GetLSHspawnZomCounter)))

(fn ZomSpawner
  (params (RoundNum :type Integer) (isRound :type Boolean))
  (if isRound
    (if (>= (Variables|Default|GetLSHRoundZomNum) (Variables|Default|GetLSHspawnZomCounter))
      ;[1 1 1] 10초에 한번 빠른좀비생성
      (if (>= (Variables|Default|GetLSHround) 3)
        (if (== (Math|Integer|%(Integer) (Variables|Default|GetLSH_TimeCounter) 10) 0)
          (CallFunction|MobMaker "/Game/SH_AI/NavigationSystem/BP_FastZom.BP_FastZom_C")
          (Development|PrintString "빠른좀비생성" true true "(R=0.141910,G=0.000000,B=1.000000,A=1.000000)"))
        ;[1 1 1] 15초에 한번 단단한좀비생성
        (if (>= (Variables|Default|GetLSHround) 5)
          (if (== (Math|Integer|%(Integer) (Variables|Default|GetLSH_TimeCounter) 15) 0)
            (CallFunction|MobMaker "/Game/SH_AI/NavigationSystem/BP_HardZom.BP_HardZom_C")
            (Development|PrintString "단단한좀비생성" true true "(R=1.000000,G=0.821324,B=0.000000,A=1.000000)"))))
      (for _index (range 0 1)
        (CallFunction|MobMaker "/Game/SH_AI/NavigationSystem/BP_Zom.BP_Zom_C")))))

(fn FastZomSpawner
  (params (RoundNum :type Integer) (isRound :type Boolean))
  (bind _lshspawnzomcounter (Variables|Default|GetLSHspawnZomCounter))
  (if (>= RoundNum 3)
    ;[1 1 1] 일반좀비 50+라운드수*10
    (if isRound
      (Variables|Default|SetLSHRoundZomNum (+ (* RoundNum 24) (Variables|Default|GetLSHDefaultZomNum)))
      (if (>= (Variables|Default|GetLSHRoundZomNum) (Variables|Default|GetLSHspawnZomCounter))
        (for _index (range 0 2)
          (CallFunction|MobMaker "/Game/SH_AI/NavigationSystem/BP_Zom.BP_Zom_C")
          (Math|Integer|IncrementInt _lshspawnzomcounter
            (:%20%20
              (Development|PrintString (Utilities|String|ToString(Integer) _lshspawnzomcounter)))))))))