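; BP_FastZom is a zombie enemy character that chases and melee-attacks the player.
; Tick re-issues a simple move toward the player's pawn until in close range, then applies damage after a short delay if still in range.
; Taking damage launches it backward and reduces health; at zero it destroys itself and increments the GI_GI game instance's dead-zombie counter.
; Several disconnected movement experiments remain unused.
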(event Custom|MoveToActorTest
  (AI|Navigation|SimpleMovetoActor (AI|GetAIController self) (Pawn|GetControlledPawn (Game|GetPlayerController 0))))

(event EventBeginPlay)

(event Game|Damage|EventAnyDamage
  (params (Damage :type Float%20%28single-precision%29) (DamageType :type Damage%20Type%20Object%20Reference) (InstigatedBy :type Controller%20Object%20Reference) (DamageCauser :type Actor%20Object%20Reference))
  (Character|LaunchCharacter (* (Transformation|GetActorForwardVector) -1000) true false)
  (Variables|Default|SetLSHZomhealth (- (Variables|Default|GetLSHZomhealth) Damage))
  (if (<= (Variables|Default|GetLSHZomhealth) 0.0)
    (Development|PrintString "dead")
    (Actor|DestroyActor)
    (bind _asgi_gi (Utilities|Casting|CastToGI_GI (Game|GetGameInstance)))
    (Math|Integer|IncrementInt (Variables|/Game/SH_AI/HUD/GI_GI.GI_GI_C|GetLSH_GI_DeadZomCounter _asgi_gi))
    (else
      (Development|PrintString (Utilities|String|ToString(Float) (Variables|Default|GetLSHZomhealth))))))

(event EventTick
  (params (DeltaSeconds :type Float%20%28single-precision%29))
  (bind _returnvalue (Game|Player|GetPlayerPawn 0))
  (if (<= (Transformation|GetDistanceTo self (Game|Player|GetPlayerPawn 0)) 1e+02)
    (Development|PrintString "zombie attack")
    (Utilities|FlowControl|Delay 0.5)
    (if (<= (Transformation|GetDistanceTo self _returnvalue) 1e+02)
      (Game|Damage|ApplyDamage _returnvalue 1e+01 0 0)
      (Development|PrintString "Hit"))
    (else
      (CallFunction|MovetoActorTest))))

(fn ConstructionScript)