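; Zombie enemy Blueprint that chases the player, attacks at close range and pays out coins when killed.
; Tick runs zomAI, which either applies delayed, range-rechecked damage or moves toward the player unless attacking, hit or dead.
; AnyDamage knocks it back and lowers health; damage arriving at zero health or below awards coins, increments the GameInstance kill counter and destroys it after a delay.
; LSHZomKill duplicates the reward and death-flag logic.
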(event Custom|zomAI
  (bind _returnvalue (Game|Player|GetPlayerPawn 0))
  (if (<= (Transformation|GetDistanceTo self (Game|Player|GetPlayerPawn 0)) 2e+02)
    (Variables|Default|SetLSH_IsAttack true)
    (if true
      (Utilities|FlowControl|Delay 1.5)
      (if (<= (Transformation|GetDistanceTo self _returnvalue) 2e+02)
        (Game|Damage|ApplyDamage _returnvalue 1e+01 0 0))
      (Utilities|FlowControl|Delay 1.2)
      (Variables|Default|SetLSH_IsAttack false))
    (elif (not (Variables|Default|GetLSH_IsAttack))
      (if (not (Variables|Default|GetLSH_IsDead))
        (if (not (Variables|Default|GetLSH_IsHit))
          (CallFunction|MovetoActorTest))))))

(event Custom|MoveToActorTest
  (AI|Navigation|SimpleMovetoActor (AI|GetAIController self) (Pawn|GetControlledPawn (Game|GetPlayerController 0))))

(event EventBeginPlay)

(event Game|Damage|EventAnyDamage
  (params (Damage :type Float%20%28single-precision%29) (DamageType :type Damage%20Type%20Object%20Reference) (InstigatedBy :type Controller%20Object%20Reference) (DamageCauser :type Actor%20Object%20Reference))
  (bind _self self)
  (bind _returnvalue (AI|GetAIController _self))
  (if (<= (Variables|Default|GetLSHZomhealth) 0.0)
    (bind _asbp_player (Utilities|Casting|CastToBP_Player (Game|GetPlayerCharacter 0)))
    (Variables|/Game/Taejeong/Blueprints/BP_Player.BP_Player_C|SetCoin _asbp_player (+ (Variables|/Game/Taejeong/Blueprints/BP_Player.BP_Player_C|GetCoin _asbp_player) 5))
    (bind _asgi_gi (Utilities|Casting|CastToGI_GI (Game|GetGameInstance)))
    (Math|Integer|IncrementInt (Variables|/Game/SH_AI/HUD/GI_GI.GI_GI_C|GetLSH_GI_DeadZomCounter _asgi_gi)
      (:%20%20
        (Variables|Default|SetLSH_IsDead true)
        (AI|Navigation|SimpleMovetoActor _returnvalue _returnvalue)
        (Collision|SetCollisionEnabled (Variables|Collision|GetCapsuleComponent) "NoCollision")
        (Utilities|FlowControl|Delay 5.0)
        (Actor|DestroyActor)))
    (else
      (Character|LaunchCharacter (* (Transformation|GetActorForwardVector) -1000) true false)
      (Variables|Default|SetLSH_IsHit true)
      (Variables|Default|SetLSHZomhealth (- (Variables|Default|GetLSHZomhealth) Damage))
      (Utilities|FlowControl|Delay 1.5)
      (Variables|Default|SetLSH_IsHit false))))

(event EventTick
  (params (DeltaSeconds :type Float%20%28single-precision%29))
  (if (Utilities|IsValid (Game|GetPlayerCharacter 0))
    (CallFunction|ZomAI)))

(fn ConstructionScript)

(fn LSHZomKill
  (bind _asbp_player (Utilities|Casting|CastToBP_Player (Game|GetPlayerCharacter 0)))
  (Variables|/Game/Taejeong/Blueprints/BP_Player.BP_Player_C|SetCoin _asbp_player (+ (Variables|/Game/Taejeong/Blueprints/BP_Player.BP_Player_C|GetCoin _asbp_player) 5))
  (bind _asgi_gi (Utilities|Casting|CastToGI_GI (Game|GetGameInstance)))
  (Math|Integer|IncrementInt (Variables|/Game/SH_AI/HUD/GI_GI.GI_GI_C|GetLSH_GI_DeadZomCounter _asgi_gi)
    (:%20%20
      (Variables|Default|SetLSH_IsDead true))))