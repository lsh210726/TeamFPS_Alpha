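; BP_MobSpawner_2 is a round-based zombie spawner that alternates timed rounds with preparation breaks.
; Tick accumulates time to flip phases, raising the round number and zombie quota at round start, then destroying every BP_Zom and resetting the spawn count at round end.
; During rounds, MobSpawn runs every tick, spawning batches with default controllers at random reachable nearby points until the count exceeds the quota.
; Debug prints report round changes and counts.
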(event Custom|MobSpawn
  (bind _lshspawnzomcounter (Variables|Default|GetLSHspawnZomCounter))
  ;[1 1 1] 라운드 참이고 라운드좀비총수 >= 스폰좀비수면 좀비 10 소환
  (if (Variables|Default|GetLSHIsRound)
    (if (>= (Variables|Default|GetLSHRoundZomNum) (Variables|Default|GetLSHspawnZomCounter))
      (for _index (range 0 (Variables|Default|GetLSHspawnNum))
        (bind _returnvalue (Game|SpawnActorfromClass "/Game/SH_AI/NavigationSystem/BP_Zom.BP_Zom_C" (Math|Conversions|ToTransform(Vector) (.RandomLocation (AI|Navigation|GetRandomReachablePointinRadius (Transformation|GetActorLocation) 5e+02 0 0))) "Undefined" "MultiplyWithRoot" 0 0))
        (Pawn|SpawnDefaultController _returnvalue)
        (Math|Integer|IncrementInt _lshspawnzomcounter
          (:%20%20
            (Development|PrintString (Utilities|String|ToString(Integer) _lshspawnzomcounter))))))))

(event EventBeginPlay)

(event Collision|EventActorBeginOverlap
  (params (OtherActor :type Actor%20Object%20Reference)))

(event EventTick
  (params (DeltaSeconds :type Float%20%28single-precision%29))
  (Variables|Default|SetLSH_currentTime (+ (Variables|Default|GetLSH_currentTime) DeltaSeconds))
  (CallFunction|MobSpawn)
  (if (< (Variables|Default|GetLSH_Timer) (Variables|Default|GetLSH_currentTime))
    (if (Variables|Default|GetLSHIsRound)
      ;[1 1 1] 만약 라운드가 참이고 시간이 종료되었다면 라운드를 종료시키고 준비시간 30초 카운트
      (Variables|Default|SetLSH_currentTime 0.0)
      (Variables|Default|SetLSH_Timer 5.0)
      (Variables|Default|SetLSHIsRound false)
      (bind _outactors (Actor|GetAllActorsOfClass "/Game/SH_AI/NavigationSystem/BP_Zom.BP_Zom_C"))
      (Actor|DestroyActor _outactors)
      (Development|PrintString "라운드 종료")
      (Variables|Default|SetLSHspawnZomCounter 0)
      (else
        ;[1 1 1] 만약 라운드가 거짓이고 시간이 종료되었다면 라운드를 1증가시키고 시작시키고 라운드시간 60초 카운트
        (Variables|Default|SetLSH_currentTime 0.0)
        (Variables|Default|SetLSH_Timer 15.0)
        (Variables|Default|SetLSHIsRound true)
        (Variables|Default|SetLSHRoundZomNum (+ (Variables|Default|GetLSHRoundZomNum) 15))
        (bind _result (Math|Integer|IncrementInt (Variables|Default|GetLSHround))
          (:%20%20
            (Development|PrintString (Utilities|String|Append (Utilities|String|ToString(Integer) _result) " 라운드 시작"))
            (Development|PrintString (Utilities|String|ToString(Integer) (Variables|Default|GetLSHRoundZomNum)))))))))

(fn ConstructionScript)

(fn RoundStart
  (Variables|Default|SetLSHIsRound true)
  (CallFunction|MobSpawn))