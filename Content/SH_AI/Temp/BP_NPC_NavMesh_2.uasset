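; A test zombie NPC that chases the player through its AI controller and mocks up a melee attack.
; After a five-second spawn timer, Tick either reissues MoveToActor or, within range, prints attack messages around a delayed distance recheck, dealing no damage.
; Taking damage launches it backward, lowers its health and destroys it at zero.
; Unconnected nodes hold alternative movement approaches.
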(event Custom|MoveToActorTest
  (AI|Navigation|MovetoActor (AI|GetAIController self) (Pawn|GetControlledPawn (Game|GetPlayerController 0)) 1e+02 true true true 0))

(event EventBeginPlay)

(event Game|Damage|EventAnyDamage
  (params (Damage :type Float%20%28single-precision%29) (DamageType :type Damage%20Type%20Object%20Reference) (InstigatedBy :type Controller%20Object%20Reference) (DamageCauser :type Actor%20Object%20Reference))
  (Character|LaunchCharacter (* (Transformation|GetActorForwardVector) -2000) true false)
  (Variables|Default|SetLSHZomhealth (- (Variables|Default|GetLSHZomhealth) Damage))
  (if (<= (Variables|Default|GetLSHZomhealth) 0.0)
    (Development|PrintString "dead")
    (Actor|DestroyActor)
    (else
      (Development|PrintString (Utilities|String|ToString(Float) (Variables|Default|GetLSHZomhealth))))))

(event EventTick
  (params (DeltaSeconds :type Float%20%28single-precision%29))
  (bind _output_get (Variables|Default|SetLSHspawnTimer (+ (Variables|Default|GetLSHspawnTimer) DeltaSeconds)))
  (if (> _output_get 5.0)
    (if (<= (Transformation|GetDistanceTo self (Game|Player|GetPlayerPawn 0)) 1.5e+02)
      (Development|PrintString "zombie attack")
      (Utilities|FlowControl|Delay 0.5)
      (if (<= (Transformation|GetDistanceTo self (Game|Player|GetPlayerPawn 0)) 1.5e+02)
        (Development|PrintString "ouch"))
      (else
        (CallFunction|MovetoActorTest)))))

(fn ConstructionScript)