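; Zombie NPC character that chases the player over the navmesh, with placeholder attack logic.
; Each Tick it re-issues a simple AI move toward the player pawn, or only prints an attack message when within close range.
; Damage launches it backward along its facing, reduces its health, and destroys it at zero.
; Disconnected leftovers include AIMoveTo and SetActorLocation experiments.
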(event Custom|MoveToActorTest
  (AI|Navigation|SimpleMovetoActor (AI|GetAIController self) (Pawn|GetControlledPawn (Game|GetPlayerController 0))))

(event EventBeginPlay)

(event Game|Damage|EventAnyDamage
  (params (Damage :type Float%20%28single-precision%29) (DamageType :type Damage%20Type%20Object%20Reference) (InstigatedBy :type Controller%20Object%20Reference) (DamageCauser :type Actor%20Object%20Reference))
  (Character|LaunchCharacter (* (Transformation|GetActorForwardVector) -1000) true false)
  (Variables|Default|SetLSHZomhealth (- (Variables|Default|GetLSHZomhealth) Damage))
  (if (<= (Variables|Default|GetLSHZomhealth) 0.0)
    (Development|PrintString "dead")
    (Actor|DestroyActor)
    (else
      (Development|PrintString (Utilities|String|ToString(Float) (Variables|Default|GetLSHZomhealth))))))

(event EventTick
  (params (DeltaSeconds :type Float%20%28single-precision%29))
  (if (<= (Transformation|GetDistanceTo self (Game|Player|GetPlayerPawn 0)) 1e+02)
    (Development|PrintString "zombie attack")
    (else
      (CallFunction|MovetoActorTest))))

(fn ConstructionScript)