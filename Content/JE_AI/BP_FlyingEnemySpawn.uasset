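; Spawner actor that runs timed rounds of flying enemies, alternating active rounds with short breaks.
; Tick accumulates time to toggle rounds, raising the enemy quota at start, then clearing it and destroying all BP_FlyingEnemyAI at end.
; Each Tick also calls the spawn routine, which creates AI-controlled batches above the spawner at random Y offsets while the spawn counter is within quota.
; That counter never resets between rounds; debug prints report progress.
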(event Custom|Fly_MobSpawn
  (bind _fly_roundflycounter (Variables|Default|GetFly_RoundFlyCounter))
  ;[1 1 1] 여러 개의 적이 스폰되지만 모습이 제대로 나타나지 않는다.
  ;;[1 1 1] FlyMobSpawn
  (if (Variables|Default|GetFly_RoundStart)
    (if (>= (Variables|Default|GetFly_RoundFlyEnemyNum) (Variables|Default|GetFly_RoundFlyCounter))
      (for _index (range 0 (Variables|Default|GetFly_SpawnNum))
        (bind _returnvalue (Game|SpawnActorfromClass "/Game/JE_AI/BP_FlyingEnemyAI.BP_FlyingEnemyAI_C" (Math|Conversions|ToTransform(Vector) (+ (Transformation|GetActorLocation) (Math|Vector|MakeVector 0.0 (Math|Random|RandomFloatinRange -1e+03 1e+03) 5e+02))) "Undefined" "MultiplyWithRoot" 0 0))
        (Pawn|SpawnDefaultController _returnvalue)
        (Math|Integer|IncrementInt _fly_roundflycounter
          (:%20%20
            (Development|PrintString (Utilities|String|ToString(Integer) _fly_roundflycounter) true true "(R=1.000000,G=0.054167,B=0.250427,A=1.000000)")))))))

(event EventBeginPlay
  ;[1 1 1] 시작 위치 변수에 대입
  (bind _output_get (Variables|Default|SetFly_SpawnLocation (Transformation|GetActorLocation))))

(event EventTick
  (params (DeltaSeconds :type Float%20%28single-precision%29))
  ;[1 1 1] 여러 개의 적이 스폰되지만 모습이 제대로 나타나지 않는다.
  ;;[1 1 1] 라운드 시작 및 적 스폰
  (Variables|Default|SetFly_CurrentTime (+ (Variables|Default|GetFly_CurrentTime) DeltaSeconds))
  (CallFunction|FlyMobSpawn)
  (if (< (Variables|Default|GetFly_Timeflow) (Variables|Default|GetFly_CurrentTime))
    (if (Variables|Default|GetFly_RoundStart)
      ;;[1 1 1] 만약 라운드가 참이고 시간이 종료되었다면 라운드를 종료시키고 준비시간 30초 카운트
      (Variables|Components|SetFly_Current%20Time 0.0)
      (Variables|Default|SetFly_Timeflow 5.0)
      (Variables|Default|SetFly_RoundStart false)
      (bind _outactors (Actor|GetAllActorsOfClass "/Game/JE_AI/BP_FlyingEnemyAI.BP_FlyingEnemyAI_C"))
      (Actor|DestroyActor _outactors)
      (Development|PrintString "라운드 종료" true true "(R=1.000000,G=0.054480,B=0.250158,A=1.000000)")
      (Variables|Default|SetFly_RoundFlyEnemyNum 0)
      (else
        ;;[1 1 1] 만약 라운드가 거짓이고 시간이 종료되었다면 라운드를 1증가시키고 시작시키고 라운드시간 60초 카운트
        (Variables|Components|SetFly_Current%20Time 0.0)
        (Variables|Default|SetFly_Timeflow 15.0)
        (Variables|Default|SetFly_RoundStart true)
        (Variables|Default|SetFly_RoundFlyEnemyNum (+ (Variables|Default|GetFly_RoundFlyEnemyNum) 5))
        (bind _result (Math|Integer|IncrementInt (Variables|Default|GetFly_RoundNum))
          (:%20%20
            (Development|PrintString (Utilities|String|Append (Utilities|String|ToString(Integer) _result) "라운드 시작") true true "(R=1.000000,G=0.054480,B=0.250158,A=1.000000)")
            (Development|PrintString (Utilities|String|ToString(Integer) (Variables|Default|GetFly_RoundFlyEnemyNum)) true true "(R=1.000000,G=0.054480,B=0.250158,A=1.000000)")))))))

(fn ConstructionScript)