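; Flying enemy character that chases and damages the player.
; Tick steers it by direct SetActorLocation along a normalized direction to the player, holding spawn height beyond 500 units and moving in full 3D when closer.
; Overlapping the player applies damage, then calls an upward launch immediately followed by a movement stop and a delay with nothing after it.
; AnyDamage lowers clamped health and triggers death at zero; AIMoveTo and event bindings are unconnected.
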(event Custom|Fly_Dead
  ;[1 1 1] FlyDamaged
  (Pawn|Components|CharacterMovement|DisableMovement (Variables|Character|GetCharacterMovement))
  (Actor|DestroyActor))

(event Custom|OnActorHit_Event
  (params (SelfActor :type Actor%20Object%20Reference) (OtherActor :type Actor%20Object%20Reference) (NormalImpulse :type Vector) (Hit :type Hit%20Result%20Structure%20%28by%20ref%29)))

(event EventBeginPlay
  ;[1 1 1] 라운드 시작, 적 계속 spawn
  ;;[1 1 1] 태어났을 때 나는 상태
  (Pawn|Components|CharacterMovement|SetMovementMode (Variables|Character|GetCharacterMovement) "MOVE_Flying" 0)
  (bind _output_get (Variables|Default|SetStartLocation (Transformation|GetActorLocation)))
  (Development|PrintString (Utilities|String|ToString(Vector) _output_get)))

(event EventTick
  (params (DeltaSeconds :type Float%20%28single-precision%29))
  (bind _returnvalue (Transformation|GetActorLocation))
  (bind _speed (Variables|Default|GetSpeed))
  (bind _direction (Variables|Default|GetDirection))
  (bind _returnvalue_2 (* _speed _direction))
  (bind _returnvalue_3 (* _returnvalue_2 DeltaSeconds))
  (bind _returnvalue_4 (+ _returnvalue _returnvalue_3))
  ;[1 1 1] 적 ai가 플레이어의 위치를 찾아서 따라가는 기능
  (Class|SkeletalMeshComponent|SetEnableBodyGravity (Variables|Character|GetMesh) false "None")
  (Variables|Default|SetTarget (Game|GetPlayerCharacter 0))
  (if (> (Transformation|GetDistanceTo (Variables|Default|GetTarget)) 5e+02)
    (Variables|Default|SetTarget (Game|GetPlayerCharacter 0))
    (CallFunction|FindTargetDirection)
    (Transformation|SetActorLocation (Math|Vector|MakeVector (.x _returnvalue_4) (.y _returnvalue_4) (.z (Variables|Default|GetStartLocation))) false false)
    (else
      (CallFunction|FindTargetDirection)
      (Transformation|SetActorLocation (+ (Transformation|GetActorLocation) (* (* (Variables|Default|GetSpeed) (Variables|Default|GetDirection)) DeltaSeconds)) false false))))

(event Game|Damage|EventAnyDamage
  (params (Damage :type Float%20%28single-precision%29) (DamageType :type Damage%20Type%20Object%20Reference) (InstigatedBy :type Controller%20Object%20Reference) (DamageCauser :type Actor%20Object%20Reference))
  ;[1 1 1] FlyDamaged
  (bind _output_get (Variables|Default|SetHealth (Math|Float|Clamp(Float) (- (Variables|Default|GetHealth) Damage) 0.0 (Variables|Default|GetMaxHealth))))
  (if (== _output_get 0.0)
    (CallFunction|FlyDead)
    (Development|PrintString "FlyEnemyDead" true true "(R=1.000000,G=0.105184,B=0.969248,A=1.000000)")
    (else
      (Development|PrintString "FlyEnemyDamaged" true true "(R=1.000000,G=0.105184,B=0.969248,A=1.000000)"))))

(event Collision|EventActorBeginOverlap
  (params (OtherActor :type Actor%20Object%20Reference))
  ;[1 1 1] player, flyingenemy collision 지정함
  ;;[1 1 1] 플레이어와 overlap 발생했을 때
  ;[1 1 1] overlap시작 - 공격, 위로 올라가서 대기 후 다시 플레이어 따라가기
  (bind _asbp_player (Utilities|Casting|CastToBP_Player OtherActor))
  (Variables|Default|SetTarget _asbp_player)
  (Game|Damage|ApplyDamage (Variables|Default|GetTarget) 1e+01 0 0)
  (Development|PrintString "FlyingEnemyAttack!!" true true "(R=1.000000,G=0.835979,B=0.096112,A=1.000000)")
  (Character|LaunchCharacter "100.000000,100.000000,1000.000000" true true)
  (Components|Movement|StopMovementImmediately (Variables|Character|GetCharacterMovement))
  (Utilities|FlowControl|RetriggerableDelay 2e+01))

(fn ConstructionScript)

(fn FindTargetDirection
  ;[1 1 1] v
  (bind _output_get (Variables|Default|SetTarget (Game|GetPlayerCharacter 0)))
  (Utilities|IsValid (Variables|Default|GetTarget)
    (:Is%20Valid
      (bind _output_get_2 (Variables|Default|SetDirection (Math|Vector|Normalize (- (Transformation|GetActorLocation _output_get) (Transformation|GetActorLocation)))))
      (Transformation|SetActorRotation (Math|Rotator|MakeRotfromZX _output_get_2 (Transformation|GetActorForwardVector))))))

(fn OnSeePawn
  (Variables|Default|SetisSeeingPlayer? true))

(fn Collision
  (Transformation|SetActorLocation (* (Math|Vector|GetUpVector "0, 0, 0") (Variables|Default|GetSpeed)) false false))

(fn BackDirection
  (Transformation|SetActorRotation (Math|Rotator|MakeRotfromZX (Transformation|GetActorLocation) (* (Transformation|GetActorForwardVector) -1.0))))

(fn FindBackDirection
  ;[1 1 1] v
  (Variables|Default|SetDirectionBack (Math|Vector|Normalize (- (+ (Transformation|GetActorLocation) "1000.000000,1000.000000,1000.000000") (Transformation|GetActorLocation (Variables|Default|GetTarget))))))